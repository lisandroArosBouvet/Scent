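; BP_Oldman is the old man NPC, hidden at start, who follows a scripted waypoint sequence driven through his AI Blackboard.
; BeheviorEvent teleports him and sets IsActive; each step writes target location and wait time from externally set arrays.
; Index-matched steps toggle rose and anger flags on BP_AnimAntonio, though the anger case writes IsGiveRosa.
; AddStateValue advances steps, deactivating and hiding him after the last; hitbox overlap only prints debug text, and TakeSpray is empty.
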(event OnComponentBeginOverlap(HitBoxCollider)
  (params (OverlappedComponent :type Primitive%20Component%20Object%20Reference) (OtherActor :type Actor%20Object%20Reference) (OtherComp :type Primitive%20Component%20Object%20Reference) (OtherBodyIndex :type Integer) (bFromSweep :type Boolean) (SweepResult :type Hit%20Result%20Structure%20%28by%20ref%29))
  (Utilities|Casting|CastToHorrorEngineCharacter OtherActor)
  (Development|PrintString "Te esta golpeando")
  (Development|PrintString (Utilities|GetDisplayName OtherComp)))

(event Custom|GoAnimation
  (params (anim :type AnimationOldman%20Enum :default "NewEnumerator0"))
  (bind _anim (Variables|Default|GetAnim))
  (switch Utilities|FlowControl|Switch|SwitchonAnimationOldman anim
    (:NewEnumerator3
      (Variables|/Game/Scent/Characters/Antonio/Animaciones/BP_AnimAntonio.BP_AnimAntonio_C|SetisHoldRosa? _anim (not (Variables|/Game/Scent/Characters/Antonio/Animaciones/BP_AnimAntonio.BP_AnimAntonio_C|GetisHoldRosa? _anim))))
    (:NewEnumerator4
      (Variables|/Game/Scent/Characters/Antonio/Animaciones/BP_AnimAntonio.BP_AnimAntonio_C|SetisGiveRosa? _anim (not (Variables|/Game/Scent/Characters/Antonio/Animaciones/BP_AnimAntonio.BP_AnimAntonio_C|GetisGiveRosa? _anim))))
    (:NewEnumerator7
      (Variables|/Game/Scent/Characters/Antonio/Animaciones/BP_AnimAntonio.BP_AnimAntonio_C|SetisGiveRosa? _anim (not (Variables|/Game/Scent/Characters/Antonio/Animaciones/BP_AnimAntonio.BP_AnimAntonio_C|GetisEnojado? _anim))))))

(event Custom|AddStateValue
  (bind _output_get (Variables|Default|SetStateIndex (+ (Variables|Default|GetStateIndex) 1)))
  (if (> (+ (Variables|Default|GetStateIndex) 1) (Utilities|Array|Length (Variables|Default|GetTargets)))
    (AI|Components|Blackboard|SetValueasBool (AI|GetBlackboard self) (Utilities|String|StringToName (Variables|Default|GetIsActive)) false)
    (Default|Show self true)
    (else
      (CallFunction|MovementPlace _output_get))))

(event Custom|SetIndexAnims
  (params (Indexs :type Array%20of%20Integers))
  (Variables|Default|SetIndexAnim Indexs))

(event Custom|BeheviorEvent
  (params (RespawnPosition :type Vector))
  (Transformation|SetActorLocation self RespawnPosition false true)
  (AI|Components|Blackboard|SetValueasBool (AI|GetBlackboard self) (Utilities|String|StringToName (Variables|Default|GetIsActive)) true)
  (bind _output_get (Variables|Default|SetStateIndex 0))
  (CallFunction|MovementPlace _output_get))

(event Custom|SetTargets
  (params (Targets :type Array%20of%20Target%20Point%20Object%20References))
  (Variables|Default|SetTargets Targets))

(event Custom|SetTimes
  (params (TImes :type Array%20of%20Floats%20%28single-precision%29))
  (Variables|Default|SetTimes TImes))

(event Custom|SetAnimationBools
  (params (Anims :type Array%20of%20AnimationOldman%20Enums :default "NewEnumerator0"))
  (Variables|Default|SetAnimationBools Anims))

(event Custom|MovementPlace
  (params (Index :type Integer))
  (bind _self self)
  (bind _returnvalue (AI|GetBlackboard _self))
  (for (_array_element _array_index) (Variables|Default|GetIndexAnim)
    (if (== _array_element Index)
      (CallFunction|GoAnimation (Utilities|Array|Get(acopy) (Variables|Default|GetAnimationBools) _array_index))))
  (AI|Components|Blackboard|SetValueasVector _returnvalue (Utilities|String|StringToName (Variables|Default|GetLocator)) (Transformation|GetActorLocation (Utilities|Array|Get(acopy) (Variables|Default|GetTargets) Index)))
  (AI|Components|Blackboard|SetValueasFloat _returnvalue (Utilities|String|StringToName (Variables|Default|GetTimeWait)) (Utilities|Array|Get(acopy) (Variables|Default|GetTimes) Index)))

(event EventTakeSpray
  (params (Type :type SprayType%20Enum :default "NewEnumerator0")))

(event EventShow
  (params (Hide :type Boolean))
  (bind _capsulecomponent (Variables|Collision|GetCapsuleComponent))
  (bind _hitboxcollider (Variables|Default|GetHitBoxCollider))
  (Rendering|SetActorHiddenInGame self Hide)
  (if Hide
    (Collision|SetCollisionEnabled _capsulecomponent "NoCollision")
    (Collision|SetCollisionEnabled _hitboxcollider "NoCollision")
    (else
      (Collision|SetCollisionEnabled _capsulecomponent "QueryAndPhysics")
      (Collision|SetCollisionEnabled _hitboxcollider "QueryAndPhysics"))))

(event EventBeginPlay
  (Default|Show self true)
  (bind _asbp_anim_antonio (Utilities|Casting|CastToBP_AnimAntonio (Components|SkeletalMesh|GetAnimInstance (Variables|Character|GetMesh))))
  (Variables|Default|SetAnim _asbp_anim_antonio))

(fn ConstructionScript)