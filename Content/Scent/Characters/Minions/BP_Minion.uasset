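; BP_Minion is an enemy minion that kills the HorrorEngineCharacter hero when its capsule hits them.
; It caches the hero on BeginPlay, and sphere overlaps toggle its in-range and can-see flags without any line-of-sight check.
; Events set its walk speed and tint its mesh by emotional type through a dynamic material instance.
; TakeSpray destroys the minion for one specific spray type.
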(event OnComponentBeginOverlap(Sphere)
  (params (OverlappedComponent :type Primitive%20Component%20Object%20Reference) (OtherActor :type Actor%20Object%20Reference) (OtherComp :type Primitive%20Component%20Object%20Reference) (OtherBodyIndex :type Integer) (bFromSweep :type Boolean) (SweepResult :type Hit%20Result%20Structure%20%28by%20ref%29))
  (Utilities|Casting|CastToHorrorEngineCharacter OtherActor)
  (Variables|Default|SetHeroInRange true)
  (Variables|Default|SetCanSee true))

(event OnComponentEndOverlap(Sphere)
  (params (OverlappedComponent :type Primitive%20Component%20Object%20Reference) (OtherActor :type Actor%20Object%20Reference) (OtherComp :type Primitive%20Component%20Object%20Reference) (OtherBodyIndex :type Integer))
  (Utilities|Casting|CastToHorrorEngineCharacter OtherActor)
  (Variables|Default|SetHeroInRange false)
  (Variables|Default|SetCanSee false))

(event OnComponentHit(CapsuleComponent)
  (params (HitComponent :type Primitive%20Component%20Object%20Reference) (OtherActor :type Actor%20Object%20Reference) (OtherComp :type Primitive%20Component%20Object%20Reference) (NormalImpulse :type Vector :default "0, 0, 0") (Hit :type Hit%20Result%20Structure%20%28by%20ref%29))
  (bind _ashorror_engine_character (Utilities|Casting|CastToHorrorEngineCharacter OtherActor))
  (Default|Die _ashorror_engine_character))

(event Custom|ChangeColor
  (params (Type :type MinionType%20Enum :default "NewEnumerator0"))
  (bind _returnvalue (Rendering|Material|CreateDynamicMaterialInstance (Variables|Character|GetMesh) 0 "/Game/Scent/Characters/Minions/MinionsMesh/MinionColor.MinionColor" "None" :!class /Script/Engine.PrimitiveComponent))
  (switch Utilities|FlowControl|Switch|SwitchonMinionType Type
    (:NewEnumerator0
      (Rendering|Material|SetVectorParameterValue _returnvalue "Color" (Variables|Default|GetColorAgressive) :!class /Script/Engine.MaterialInstanceDynamic))
    (:NewEnumerator1
      (Rendering|Material|SetVectorParameterValue _returnvalue "Color" (Variables|Default|GetColorFearful) :!class /Script/Engine.MaterialInstanceDynamic))
    (:NewEnumerator2
      (Rendering|Material|SetVectorParameterValue _returnvalue "Color" (Variables|Default|GetColorDepressed) :!class /Script/Engine.MaterialInstanceDynamic))))

(event Custom|ChangeSpeed
  (params (Speed :type Float%20%28single-precision%29))
  (Variables|/Script/Engine.CharacterMovementComponent|SetMaxWalkSpeed (Variables|Character|GetCharacterMovement) Speed))

(event EventBeginPlay
  (bind _outactors (Actor|GetAllActorsOfClass "/Game/HorrorEngine/Blueprints/Core/HorrorEngineCharacter.HorrorEngineCharacter_C"))
  (Variables|Default|SetHero (Utilities|Array|Get(acopy) _outactors)))

(event EventTakeSpray
  (params (Type :type SprayType%20Enum :default "NewEnumerator0"))
  (if (Utilities|Enum|Equal(Enum) Type "NewEnumerator3")
    (Actor|DestroyActor)))

(fn ConstructionScript)