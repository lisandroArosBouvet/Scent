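; Thunderstorm actor that stages a looping lightning strike around the player at random intervals.
; Each cycle briefly spikes manual exposure on PPVolume by overwriting its settings, then plays a 2D thunder crack and calls Strike.
; Strike moves the actor to a random point ahead of the player's view, yawed toward them.
; The Thunder_strike timeline then animates the ThunderPlane material's Y and Emission parameters.
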(event Custom|Strike
  (bind _thunder_plane (Variables|Default|GetThunder_plane))
  (|ReLocate
    (:OutputPin
      (bind _y (Timeline|Thunder_strike PlayFromStart)
        (:Update
          (Rendering|Material|SetScalarParameterValueonMaterials _thunder_plane "Y" _y)
          (Rendering|Material|SetScalarParameterValueonMaterials _thunder_plane "Emission" (* (+ _y 1.0) 5e+01)))))))

(event EventBeginPlay
  (bind _pp_volume (Variables|Default|GetPP_volume))
  (Utilities|FlowControl|Delay (Math|Random|RandomFloatinRange 8.0 16.0) :!label _label)
  (Utilities|FlowControl|Delay 0.3)
  (bind _output_get (Variables|Default|SetOriginal%20Exposure%20Compensation (Utilities|Struct|BreakPostProcessSettings (Variables|/Script/Engine.PostProcessVolume|GetSettings _pp_volume))))
  (Variables|/Script/Engine.PostProcessVolume|SetSettings _pp_volume (Utilities|Struct|MakePostProcessSettings "AEM_Manual" 15.0))
  (Utilities|FlowControl|Delay 0.3)
  (Variables|/Script/Engine.PostProcessVolume|SetSettings _pp_volume (Utilities|Struct|MakePostProcessSettings "AEM_Manual" _output_get))
  (Audio|PlaySound2D "/Game/HorrorEngine/Audio/Effects/ThunderCrack.ThunderCrack" 1.0 1.0 0.0 0 0)
  (CallFunction|Strike)
  (goto _label))

(event Collision|EventActorBeginOverlap
  (params (OtherActor :type Actor%20Object%20Reference)))

(event EventTick
  (params (DeltaSeconds :type Float%20%28single-precision%29)))

(fn ConstructionScript)